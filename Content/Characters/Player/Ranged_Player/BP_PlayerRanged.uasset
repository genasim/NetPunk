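; BP_PlayerRanged is the dual-gun ranged player character, handling hitscan attacks, an aiming crosshair, the pause menu and its save name.
; HandleAttack picks the left or right gun, then traces from the camera to find the aim point and from that gun's muzzle to that point.
; A confirmed hit sends a Weapon.Hit gameplay event with target data to the instigator.
; The crosshair toggle removes the widget for non-local characters.
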(event `self.ReceiveBeginPlay`)

(event `InputAction|PauseMenu`
  (params (Key :type "Key Structure"))
  ;[1 1 1] Show Pause Menu
  (:`Pressed`
    (`/Engine/EditorBlueprintResources/StandardMacros.IsValid` (`self.PauseMenuREF`)
      (:`Is Valid`
        _)
      (:`Is Not Valid`
        (bind _returnvalue (`|CreateWidget` "/Game/UI/UI_PauseMenu.UI_PauseMenu_C"))
        (bind _output_get (set `self.PauseMenuREF` _returnvalue))))
    (`UserWidget.AddToViewport` _output_get 0)))

(event `/Game/Characters/Player/BI_AttackInterface.Handle Attack`
  (bind _returnvalue (`self.GetInstigator`))
  (bind _weapon (`self.Determine Weapon To Fire`))
  (bind (_outhit _returnvalue_2) (`self.Make Line Trace from Gun to Target` _weapon))
  (if _returnvalue_2
    (bind (_bblockinghit _binitialoverlap _time _distance _location _impactpoint _normal _impactnormal _physmat _hitactor) (`GameplayStatics.BreakHitResult` _outhit))
    (`AbilitySystemBlueprintLibrary.SendGameplayEventToActor` _returnvalue (struct :`TagName` "Weapon.Hit") (make `GameplayEventData` (struct) _returnvalue _hitactor null null (struct) (struct) (struct) 0.0 (`AbilitySystemBlueprintLibrary.AbilityTargetDataFromActor` _hitactor)))))

(fn `Determine Weapon To Fire`
  (returns (Weapon :type "SkeletalMeshComponent Object Reference"))
  (if (`self.FireRightWeapon`)
    (return (`self.GunRight`))
    (else
      (return (`self.GunLeft`)))))

(fn `GetUniqueSaveName`
  (returns (ReturnValue :type String))
  (return "Player_Ranged"))

(fn `Make Line Trace from Gun to Target`
  (params (Gun :type "SkeletalMeshComponent Object Reference"))
  (returns (OutHit :type "HitResult Structure") (ReturnValue :type Boolean))
  (locals (Success :type Boolean))
  (bind _camera (`self.Camera`))
  (bind _returnvalue (`SceneComponent.K2_GetComponentLocation` _camera))
  (bind (_outhit _returnvalue_2) (`KismetSystemLibrary.LineTraceSingle` :`Start` _returnvalue :`End` (+ _returnvalue (* (`KismetMathLibrary.GetForwardVector` (`SceneComponent.K2_GetComponentRotation` _camera)) (`self.Range`))) :`TraceChannel` "TraceTypeQuery1" :`DrawTime` 4.0))
  (if _returnvalue_2
    (bind (_outhit_2 _returnvalue_3) (`KismetSystemLibrary.LineTraceSingle` :`Start` (`SceneComponent.GetSocketLocation` Gun "Muzzle") :`End` (`.Location` (`GameplayStatics.BreakHitResult` _outhit)) :`TraceChannel` "TraceTypeQuery1" :`DrawDebugType` "ForDuration" :`TraceColor` (struct :`R` 1.0 :`G` 1.0 :`A` 1.0) :`TraceHitColor` (struct :`R` 1.0 :`G` 1.0 :`B` 1.0 :`A` 1.0)))
    (if _returnvalue_3
      (return _outhit_2 true)
      (else
        (return (struct) false)))
    (else
      (return (struct) false))))

(fn `Toggle Crosshair`
  (params (`Is Aiming` :type Boolean))
  (if `Is Aiming`
    (bind _returnvalue (`|CreateWidget` "/Game/UI/PlayerRanged_Crosshair.PlayerRanged_Crosshair_C"))
    (bind _output_get (set `self.Crosshair` _returnvalue))
    (`UserWidget.AddToViewport` _output_get 0)
    ;[1 1 1] Remove the crosshair from other players' screen; otherwise the ability will add it to all of them
    (if (!= (`NWGameInstance.GetLocalPlayerCharacter`) self)
      (`Widget.RemoveFromParent` (`self.Crosshair`)))
    (else
      (`Widget.RemoveFromParent` (`self.Crosshair`)))))

(fn `UserConstructionScript`)