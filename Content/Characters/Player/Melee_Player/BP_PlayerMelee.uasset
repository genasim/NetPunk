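; BP_PlayerMelee is the melee player character, identified for saving by the unique name "Player_Melee".
; HandleAttack sphere-traces for Pawns between the Start and End sockets on the right sword, with timed debug drawing.
; A hit sends a Weapon.Hit gameplay event to the instigator, carrying the struck actor as target data for the Gameplay Ability System.
; The PauseMenu input creates the pause widget once, caches it and adds it to the viewport.
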(event `self.ReceiveBeginPlay`)

(event `InputAction|PauseMenu`
  (params (Key :type "Key Structure"))
  ;[1 1 1] Show Pause Menu
  (:`Pressed`
    (`/Engine/EditorBlueprintResources/StandardMacros.IsValid` (`self.PauseMenuREF`)
      (:`Is Valid`
        _)
      (:`Is Not Valid`
        (bind _returnvalue (`|CreateWidget` "/Game/UI/UI_PauseMenu.UI_PauseMenu_C"))
        (bind _output_get (set `self.PauseMenuREF` _returnvalue))))
    (`UserWidget.AddToViewport` _output_get 0)))

(event `/Game/Characters/Player/BI_AttackInterface.Handle Attack`
  (bind _returnvalue (`self.GetInstigator`))
  (bind _swordright (`self.SwordRight`))
  (bind (_outhit _returnvalue_2) (`KismetSystemLibrary.SphereTraceSingleForObjects` (`SceneComponent.GetSocketLocation` _swordright "Start") (`SceneComponent.GetSocketLocation` _swordright "End") 21.0 (`|MakeArray` "ObjectTypeQuery3" :!type "EObjectTypeQuery Enum") false (`|MakeArray` self :!type "Actor Object Reference") "ForDuration"))
  (if _returnvalue_2
    (bind (_bblockinghit _binitialoverlap _time _distance _location _impactpoint _normal _impactnormal _physmat _hitactor) (`GameplayStatics.BreakHitResult` _outhit))
    (`AbilitySystemBlueprintLibrary.SendGameplayEventToActor` _returnvalue (struct :`TagName` "Weapon.Hit") (make `GameplayEventData` (struct) _returnvalue _hitactor null null (struct) (struct) (struct) 0.0 (`AbilitySystemBlueprintLibrary.AbilityTargetDataFromActor` _hitactor)))))

(fn `GetUniqueSaveName`
  (returns (ReturnValue :type String))
  (return "Player_Melee"))

(fn `UserConstructionScript`)