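; Player character Blueprint that handles pause menu input and saves and restores the player's transform.
; The PauseMenu action lazily creates and caches the pause widget, then adds it to the viewport.
; OnBeforeSave stores and prints the current transform, BeginPlay teleports to the stored one, and key 1 triggers SaveGame.
; GetUniqueSaveName returns an empty string, and a dodge debug check is left unconnected.
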(event `InputAction|PauseMenu`
  (params (Key :type "Key Structure"))
  ;[1 1 1] Show Pause Menu
  (:`Pressed`
    (`/Engine/EditorBlueprintResources/StandardMacros.IsValid` (`self.PauseMenuREF`)
      (:`Is Valid`
        _)
      (:`Is Not Valid`
        (bind _returnvalue (`|CreateWidget` "/Game/UI/UI_PauseMenu.UI_PauseMenu_C"))
        (bind _output_get (set `self.PauseMenuREF` _returnvalue))))
    (`UserWidget.AddToViewport` _output_get 0)))

(event `self.ReceiveTick`
  (params (DeltaSeconds :type "Float (single-precision)")))

(event `self.ReceiveBeginPlay`
  (`self.K2_SetActorTransform` (`self.Player Transform`) false true))

(event `SaveInterface.OnBeforeSave`
  (bind _output_get (set `self.Player Transform` (`self.GetTransform`)))
  (`KismetSystemLibrary.PrintString` (`KismetStringLibrary.Conv_TransformToString` _output_get) true true (struct :`G` 0.66 :`B` 1.0 :`A` 1.0) 5.0))

(event `Key|One`
  (params (Key :type "Key Structure"))
  (:`Pressed`
    (`SaveManager.SaveGame`)))

(fn `GetUniqueSaveName`
  (returns (ReturnValue :type String))
  (return ""))

(fn `UserConstructionScript`)