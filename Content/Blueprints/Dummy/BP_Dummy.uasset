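; BP_Dummy is a damageable dummy character that plays hit reactions and dies when its health runs out.
; AnyDamage passes a DoOnce gate, subtracts Health, then plays a hit-react montage and reopens the gate after that montage's length.
; At zero health it plays a death montage, disables collision and deactivates movement, leaving the gate closed.
; Montages are relayed through server and client events for replicated playback.
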(event `self.ReceiveAnyDamage`
  (params (Damage :type "Float (single-precision)") (DamageType :type "DamageType Object Reference") (InstigatedBy :type "Controller Object Reference") (DamageCauser :type "Actor Object Reference"))
  (`/Engine/EditorBlueprintResources/StandardMacros.DoOnce` false :!label _label
    (:`Completed`
      (bind _output_get (set `self.Health` (- (`self.Health`) Damage)))
      (if (<= _output_get 0.0)
        (`self.Run Replicated AnimMontage` "/Game/Animations/Attack/Death_Montage.Death_Montage")
        (`self.SetActorEnableCollision` false)
        (`ActorComponent.Deactivate` (`self.CharacterMovement`))
        (else
          (`self.Run Replicated AnimMontage` "/Game/Animations/Attack/HitReact_Montage.HitReact_Montage")
          (`KismetSystemLibrary.Delay` (`self.Delay`))
          (goto _label :!via `Reset`))))))

(event `Run Replicated AnimMontage`
  (params (AnimMontage :type "AnimMontage Object Reference"))
  (`self.Run AnimMontage on Server` AnimMontage))

(event `Run AnimMontage on Server`
  (params (AnimMontage :type "AnimMontage Object Reference"))
  (`self.Run AnimMontage on Clients` AnimMontage))

(event `Run AnimMontage on Clients`
  (params (AnimMontage :type "AnimMontage Object Reference"))
  (bind _returnvalue (`self.PlayAnimMontage` AnimMontage))
  (set `self.Delay` _returnvalue))

(fn `UserConstructionScript`)