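; BP_NetGameGameMode is a game mode that assigns different pawn classes to players in a networked game.
; Its GetDefaultPawnClassForController override gives BP_PlayerMelee to the controller owning player state index 0 and BP_PlayerRanged to every other player controller.
; The DefaultPawnClass fallback sits behind a validity check that follows the PlayerController cast, so a failed cast stops before reaching it.
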(fn `GetDefaultPawnClassForController`
  (params (InController :type "Controller Object Reference"))
  (returns (ReturnValue :type "Object Class Reference"))
  (locals (`Player Controller` :type "PlayerController Object Reference"))
  (bind _asplayer_controller (cast `PlayerController` InController))
  (bind _output_get (set `local.Player Controller` _asplayer_controller))
  (`/Engine/EditorBlueprintResources/StandardMacros.IsValid` _output_get
    (:`Is Valid`
      (if (== (`PlayerState.GetPlayerController` (`GameplayStatics.GetPlayerState` 0)) (`local.Player Controller`))
        (return "/Game/Characters/Player/Melee_Player/BP_PlayerMelee.BP_PlayerMelee_C")
        (else
          (return "/Game/Characters/Player/Ranged_Player/BP_PlayerRanged.BP_PlayerRanged_C"))))
    (:`Is Not Valid`
      (return (`self.DefaultPawnClass`)))))

(fn `UserConstructionScript`)